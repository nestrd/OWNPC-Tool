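; Parent character Blueprint with a flipbook sprite, driven by a two-level state machine.
; A superstate change (idle, move or action) swaps the sprite's flipbook and resets all substates to their first value.
; Each tick, the sprite's yaw eases toward left or right based on the sign of Y velocity, so it turns smoothly.
; When stopped, it keeps rotating only until it is near either side-facing angle.
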(event `UpdateSuperstate`
  (params (newSuperstate :type "/Game/AI/States/state_Superstates Enum" :default "NewEnumerator0"))
  (bind _output_get (set `self.currentSuperstate` newSuperstate))
  (`PaperFlipbookComponent.SetFlipbook` (`self.CharacterSprite`) (select `/Game/AI/States/state_Superstates` (`self.currentSuperstate`) :`NewEnumerator0` "/Game/Characters/Animations/FB_CharacterIdle.FB_CharacterIdle" :`NewEnumerator1` "/Game/Characters/Animations/FB_CharacterMove.FB_CharacterMove" :`NewEnumerator2` "/Game/Characters/Animations/FB_CharacterDoAction.FB_CharacterDoAction" :!type "PaperFlipbook Object Reference"))
  (`self.ResetSubstates`)
  (switch `/Game/AI/States/state_Superstates` _output_get
    (:`NewEnumerator0`
      (`self.UpdateSubstate_Idle` "NewEnumerator0"))
    (:`NewEnumerator1`
      (`self.UpdateSubstate_Move` "NewEnumerator0"))
    (:`NewEnumerator2`
      (`self.UpdateSubstate_Action` "NewEnumerator0"))))

(event `UpdateSubstate_Idle`
  (params (newSubstate :type "/Game/AI/States/state_Substates_Idle Enum" :default "NewEnumerator0"))
  ;[1 1 1] Substates
  (set `self.currentIdleState` newSubstate))

(event `UpdateSubstate_Move`
  (params (newSubstate :type "/Game/AI/States/state_Substates_Move Enum" :default "NewEnumerator0"))
  ;[1 1 1] Substates
  (set `self.currentMoveState` newSubstate))

(event `self.ReceiveTick`
  (params (DeltaSeconds :type "Float (single-precision)"))
  ;[0.2655 1 0.1643] Tick Event
  (`self.RotateSpriteToDirection` DeltaSeconds))

(event `UpdateSubstate_Action`
  (params (newSubstate :type "/Game/AI/States/state_Substates_Action Enum" :default "NewEnumerator0"))
  ;[1 1 1] Substates
  (set `self.currentActionState` newSubstate))

(fn `ResetSubstates`
  (`self.UpdateSubstate_Idle` "NewEnumerator0")
  (`self.UpdateSubstate_Move` "NewEnumerator0")
  (`self.UpdateSubstate_Action` "NewEnumerator0"))

(fn `RotateSpriteToDirection`
  (params (Alpha :type "Float (single-precision)"))
  (bind (_returnvalue_x _returnvalue_y) (`KismetMathLibrary.BreakVector` (`self.GetVelocity`)))
  (bind _returnvalue (`SceneComponent.K2_GetComponentRotation` (`self.CharacterSprite`)))
  (if (!= (`self.GetVelocity`) (0.0 0.0 0.0) :`ErrorTolerance` 0.1)
    (`SceneComponent.K2_SetWorldRotation` (`self.CharacterSprite`) (`KismetMathLibrary.RLerp` (`SceneComponent.K2_GetComponentRotation` (`self.CharacterSprite`)) (`KismetMathLibrary.MakeRotator` 0.0 0.0 (select `bool` (< _returnvalue_y 0.0) :`false` 90.0 :`true` -90.0 :!type "Float (single-precision)")) (* Alpha 10.0)) false false :!label _label)
    (elif (not (or (== _returnvalue (struct :`Yaw` -90.0) :`ErrorTolerance` 10.0) (== _returnvalue (struct :`Yaw` 90.0) :`ErrorTolerance` 10.0)))
      (goto _label))))

(fn `UserConstructionScript`)